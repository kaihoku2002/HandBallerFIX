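; CPU opponent character for a ball-throwing, tackling goal game, which returns to its start position and pauses briefly after either side scores.
; BeginPlay caches the goal and player, clears GameInstance possession flags and binds both goal events.
; An MCPUState switch (Chase, Go, Pass) handles AI movement, socket-attached ball pickup and impulse throws, alongside cooldown-gated tackles that swap possession.
; That gameplay graph is disconnected: Tick is empty, so none of it runs.
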(event `self.ReceiveTick`
  (params (DeltaSeconds :type "Float (single-precision)")))

(event `self.ReceiveBeginPlay`
  (bind _asgame_instance_bp2 (cast `/Game/Instance/GameInstance_BP2` (`GameplayStatics.GetGameInstance`) :!pure true))
  (`|ExecutionSequence`
    (:`then_0`
      ;[1 1 1] ゴールオブジェクトゲッチュー　担当：坂田
      (bind _returnvalue (`GameplayStatics.GetActorOfClass` "/Game/BP/GoalObjectBP.GoalObjectBP_C"))
      (set `self.goal` _returnvalue)
      (set `/Game/Instance/GameInstance_BP2.CPU_HasBall` false _asgame_instance_bp2)
      (set `/Game/Instance/GameInstance_BP2.Member_HasBall` false _asgame_instance_bp2)
      (set `/Game/Instance/GameInstance_BP2.Has Ball` false _asgame_instance_bp2))
    (:`then_1`
      ;[1 1 1] ゴール時処理　担当：坂田
      (set `self.First Pos` (`self.K2_GetActorLocation`)))
    (:`then_2`
      (add `/Game/BP/MyGoalObject.M Goal` (`self.MGoal`) (delegate `Player Goal`)))
    (:`then_3`
      (add `/Game/BP/GoalObjectBP.E Goal` (`self.EGoal`) (delegate `Enemy Goal`)))
    (:`then_4`
      (bind _outactors (`GameplayStatics.GetAllActorsOfClass` "/Game/BP/MyCharacterBP.MyCharacterBP_C"))
      (for (_array_element _array_index) _outactors
        (if (== _array_index 0)
          (set `self.HitPlayer` _array_element))))))

(event `Player Goal`
  ;[1 1 1] ゴール時処理　担当：坂田
  (`self.K2_SetActorLocation` (`self.First Pos`))
  (`CharacterMovementComponent.DisableMovement` (`self.CharacterMovement`))
  (`KismetSystemLibrary.Delay` 6.0)
  (`CharacterMovementComponent.SetMovementMode` (`self.CharacterMovement`) "MOVE_Walking" 0)
  (set `self.m_CPUState` "CPUS_Chase"))

(event `Enemy Goal`
  ;[1 1 1] ゴール時処理　担当：坂田
  (`self.K2_SetActorLocation` (`self.First Pos`))
  (`CharacterMovementComponent.DisableMovement` (`self.CharacterMovement`))
  (`KismetSystemLibrary.Delay` 6.0)
  (`CharacterMovementComponent.SetMovementMode` (`self.CharacterMovement`) "MOVE_Walking" 0)
  (set `self.m_CPUState` "CPUS_Chase"))

(fn `Overlap Member`
  (bind _returnvalue (`GameplayStatics.GetActorOfClass` null))
  (if (< (`self.GetDistanceTo` _returnvalue) 300.0)
    (set `self.Member Check` true)))

(fn `Overlap Player`
  (locals (NewLocalVar_0 :type Boolean))
  (bind _returnvalue (`GameplayStatics.GetActorOfClass` "/Game/BP/MyCharacterBP.MyCharacterBP_C"))
  (if (< (`self.GetDistanceTo` _returnvalue) 300.0)
    (set `self.PlayerCheck` true)))

(fn `UserConstructionScript`)