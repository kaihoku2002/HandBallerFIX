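; Player character Blueprint for a goal-based ball game, with tackle, jump montage and throw trigger inputs.
; Goal events reset it to its spawn point and briefly freeze movement, as at match start.
; Tick drives tackle overlap checks against CPU-tagged actors and frame-counted tackle duration and cooldown.
; Catch, throw physics and slope boost graphs are disconnected; trace-based foot IK and ground-height helpers are defined but not called here.
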(event `self.ReceiveBeginPlay`
  (bind _charactermovement (`self.CharacterMovement`))
  (`|ExecutionSequence`
    (:`then_0`
      (set `self.First Pos` (`self.K2_GetActorLocation`)))
    (:`then_1`
      ;[1 1 1] ゴール時処理　担当：坂田
      (add `/Game/BP/GoalObjectBP.E Goal` (`self.EGoal`) (delegate `EnemyGoal`)))
    (:`then_2`
      (add `/Game/BP/MyGoalObject.M Goal` (`self.MGoal`) (delegate `PlayerGoal`)))
    (:`then_3`
      ;[1 1 1] スタート時　担当：坂田
      (if (not (`/Game/Instance/GameInstance_BP2.StartFlag` (cast `/Game/Instance/GameInstance_BP2` (`GameplayStatics.GetGameInstance`) :!pure true)))
        (set `self.m_bCanControl` false)
        (`CharacterMovementComponent.DisableMovement` (`self.CharacterMovement`))
        (`KismetSystemLibrary.Delay` 6.0)
        (`CharacterMovementComponent.SetMovementMode` _charactermovement "MOVE_Walking" 0)
        (if (not (`NavMovementComponent.IsFalling` _charactermovement))
          (set `self.m_bCanControl` true))))))

(event `EnemyGoal`
  ;[1 1 1] ゴール時処理　担当：坂田
  (`self.K2_SetActorLocation` (`self.First Pos`))
  (`CharacterMovementComponent.DisableMovement` (`self.CharacterMovement`))
  (`KismetSystemLibrary.Delay` 6.0)
  (`CharacterMovementComponent.SetMovementMode` (`self.CharacterMovement`) "MOVE_Walking" 0))

(event `PlayerGoal`
  ;[1 1 1] ゴール時処理　担当：坂田
  (`self.K2_SetActorLocation` (`self.First Pos`))
  (`CharacterMovementComponent.DisableMovement` (`self.CharacterMovement`))
  (`KismetSystemLibrary.Delay` 6.0)
  (`CharacterMovementComponent.SetMovementMode` (`self.CharacterMovement`) "MOVE_Walking" 0))

(event `InputAction|Throw`
  (params (Key :type "Key Structure"))
  ;[0 1 0.1412 1 30] 投げる処理　担当：海北
)

(event `self.ReceiveTick`
  (params (DeltaSeconds :type "Float (single-precision)"))
  (`|ExecutionSequence`
    (:`then_0`
      (`/Engine/EditorBlueprintResources/StandardMacros.FlipFlop`))
    (:`then_1`
      ;[1 1 1] タックルクールタイム　担当：坂本
      (if (`self.Cooldown_Tackle`)
        (`|ExecutionSequence`
          (:`then_0`
            (if (< (`self.Tackle_CoolTimeCnt`) (`self.Tackle Cool Time`))
              (set `self.Time_Tackle` (+ (`self.Time_Tackle`) 1))
              (if (== (mod (`self.Time_Tackle`) 60) 0)
                (set `self.Time_Tackle` 0)
                (set `self.Tackle_CoolTimeCnt` (+ (`self.Tackle_CoolTimeCnt`) 1)))
              (else
                ;;[1 1 1] 初期化
                (set `self.Tackle_CoolTimeCnt` 0)
                (set `self.Tackle_LifeFrame` 0)
                (set `self.Cooldown_Tackle` false))))
          (:`then_1`
            (if (`self.m_bTackle`)
              (if (< (`self.Tackle_LifeFrame`) 30)
                (bind _result (`/Engine/EditorBlueprintResources/StandardMacros.IncrementInt` (`self.Tackle_LifeFrame`))
                  (:`  `
                    (set `self.Tackle_LifeFrame` _result)))
                (else
                  (set `self.m_bTackle` false)
                  (set `self.Tackle_LifeFrame` 0))))))))
    (:`then_5`
      ;[1 1 1] タックル関連　担当：坂本
      (if (`self.TackleStart`)
        (`|ExecutionSequence`
          (:`then_0`
            (bind _outactors (`GameplayStatics.GetAllActorsWithTag` "CPU"))
            (if (`self.OverlapedSphere`)
              (goto _label :!via `Break`)
              (else
                (for _array_element _outactors :!label _label
                  (if (`PrimitiveComponent.IsOverlappingActor` (`self.m_pSphereComp`) _array_element)
                    (set `self.HitCPU` (cast `/Game/BP/CPUCharacterBP` _array_element :!pure true))
                    (set `self.OverlapedSphere` true)))
                ;;[1 1 1] タックル
                (set `self.OverlapedSphere` false)
                (`self.Tackle`))))
          (:`then_1`
            (`KismetSystemLibrary.Delay` 0.4)
            (set `self.TackleStart` false)))))
    (:`then_6`
      (`KismetSystemLibrary.DrawDebugArrow` (0.0 0.0 0.0) (0.0 0.0 0.0) 100.0 (struct :`R` 0.950145 :`G` 0.958333 :`B` 0.144825 :`A` 1.0)))))

(event `Key|Gamepad_LeftShoulder`
  (params (Key :type "Key Structure"))
  ;[0 1 0.1412 1 30] 投げる処理　担当：海北
  (:`Pressed`
    (if (`self.m_bIsHolding`)
      (set `/Game/Instance/GameInstance_BP2.Has Ball` false (cast `/Game/Instance/GameInstance_BP2` (`GameplayStatics.GetGameInstance`) :!pure true))
      (set `self.ThrowAnim` true))))

(event `InputAction|Tackle`
  (params (Key :type "Key Structure"))
  ;[1 1 1] タックル関連　担当：坂本
  ;;[1 1 1] タックルインプット
  (:`Pressed`
    (set `self.TackleStart` true)))

(event `Key|Gamepad_RightShoulder`
  (params (Key :type "Key Structure"))
  ;[0 1 0.1412 1 30] ジャンプのアニメーション再生　担当：海北
  (:`Pressed`
    (if (not (`NavMovementComponent.IsFalling` (`self.CharacterMovement`)))
      (`self.PlayAnimMontage` "/Game/Anim_Chara/JUMP_Montage1.JUMP_Montage1")
      (`GameplayStatics.PlaySound2D` "/Game/Sound/foley_jump_movement_throw_05.foley_jump_movement_throw_05" 1.0 1.0 0.0 null null))))

(event `Key|SpaceBar`
  (params (Key :type "Key Structure"))
  ;[0 1 0.1412 1 30] ジャンプのアニメーション再生　担当：海北
)

(fn `Tackle`
  (if (`self.Cooldown_Tackle`)
    _
    (elif (`self.m_bCanTackle`)
      (if (`self.m_bTackle`)
        _
        (elif (`self.m_bIsHolding`)
          _
          (elif (not (`NavMovementComponent.IsFalling` (`self.CharacterMovement`)))
            (`GameplayStatics.PlaySound2D` "/Game/Sound/tacklestart.tacklestart" 1.0 1.0 0.0 null null)
            (`self.PlayAnimMontage` "/Game/Anim_Chara/takkle_Montage.takkle_Montage")
            (set `self.m_bTackle` true)
            (set `self.Cooldown_Tackle` true)))))))

(fn `TraceFromLocation`
  (params (`From Location` :type "Vector Structure") (`To Location` :type "Vector Structure"))
  (returns (Hit :type Boolean) (Location :type "Vector Structure"))
  (bind (_outhit _returnvalue) (`KismetSystemLibrary.LineTraceSingle` `From Location` `To Location` "TraceTypeQuery1"))
  (return _returnvalue (`KismetMathLibrary.SelectVector` (`.Location` (`GameplayStatics.BreakHitResult` _outhit)) (0.0 0.0 0.0) _returnvalue)))

(fn `Try Foot Trace`
  (params (`Socket Name` :type Name) (CapsuleLowerLocationZ :type "Float (double-precision)"))
  (returns (Hit :type Boolean) (`Hit Offset` :type "Float (double-precision)") (`Sinking Distance` :type "Float (double-precision)"))
  (bind _returnvalue (`SceneComponent.GetSocketLocation` (`self.Mesh`) `Socket Name`))
  (bind _z (.z _returnvalue))
  (if (> CapsuleLowerLocationZ _z)
    (bind (_hit _location) (`self.TraceFromLocation` (`KismetMathLibrary.MakeVector` (.x _returnvalue) (.y _returnvalue) CapsuleLowerLocationZ) _returnvalue))
    (return _hit (`KismetMathLibrary.SelectFloat` (- (.z _location) CapsuleLowerLocationZ) 0.0 _hit) (`KismetMathLibrary.SelectFloat` (- (.z _location) _z) 0.0 _hit))
    (else
      (return false 0.0 0.0))))

(fn `Try Get Foot Offset`
  (params (`Location X` :type "Float (double-precision)") (`Location Y` :type "Float (double-precision)") (`From Location Z` :type "Float (double-precision)") (`To Location Z` :type "Float (double-precision)"))
  (returns (Offset :type "Float (double-precision)"))
  (locals (NewLocalVar_0 :type "ARPin Object Reference"))
  (bind (_hit _location) (`self.TraceFromLocation` (`KismetMathLibrary.MakeVector` `Location X` `Location Y` `From Location Z`) (`KismetMathLibrary.MakeVector` `Location X` `Location Y` `To Location Z`)))
  (return (`KismetMathLibrary.SelectFloat` (- (.z _location) `To Location Z`) 0.0 _hit)))

(fn `UpdateActorLocationZ`
  (params (NewParam :type "Float (double-precision)"))
  (locals (DeltaSeconds_ :type "Float (double-precision)") (CapsuleLowerLocationZ :type "Float (double-precision)") (HitOffset :type "Float (double-precision)") (SinkingDistance :type "Float (double-precision)") (LocationInterpSpeed :type "Float (double-precision)" :default 50.0))
  (bind (_returnvalue_x _returnvalue_y _returnvalue_z) (`KismetMathLibrary.BreakVector` (`self.GetVelocity`)))
  (bind _capsulecomponent (`self.CapsuleComponent`))
  (bind _returnvalue (`KismetMathLibrary.FInterpTo` (`self.Interp Sinking Distance`) (`local.SinkingDistance`) 1.0 (`local.LocationInterpSpeed`)))
  (bind (_returnvalue_x_2 _returnvalue_y_2 _returnvalue_z_2) (`KismetMathLibrary.BreakVector` (`SceneComponent.K2_GetComponentLocation` _capsulecomponent)))
  (set `local.DeltaSeconds_` NewParam)
  (if (<= _returnvalue_z 0.0)
    (`|ExecutionSequence`
      (:`then_0`
        (set `local.CapsuleLowerLocationZ` (- _returnvalue_z_2 (`CapsuleComponent.CapsuleHalfHeight` _capsulecomponent))))
      (:`then_1`
        ;[1 1 1 1 37] 左あしトレース
        (bind (_hit _hit_offset _sinking_distance) (`self.Try Foot Trace` (`self.LeftGroundSocket`) (`local.CapsuleLowerLocationZ`)))
        (if (< _hit_offset (`local.HitOffset`))
          (set `local.HitOffset` _hit_offset)
          (set `local.SinkingDistance` _sinking_distance)))
      (:`then_2`
        ;[1 1 1 1 37] 右あしトレース
        (bind (_hit_2 _hit_offset_2 _sinking_distance_2) (`self.Try Foot Trace` (`self.RightGroundSocket`) (`local.CapsuleLowerLocationZ`)))
        (if (< _hit_offset_2 (`local.HitOffset`))
          (set `local.HitOffset` _hit_offset_2)
          (set `local.SinkingDistance` _sinking_distance_2)))
      (:`then_3`
        (bind _output_get (set `self.Interp Sinking Distance` _returnvalue))
        (if (> _returnvalue 0.0)
          (`self.K2_AddActorLocalOffset` (`KismetMathLibrary.MakeVector` 0.0 0.0 _output_get))
          (`CharacterMovementComponent.SetMovementMode` (`self.CharacterMovement`) "MOVE_Walking" 0))))))

(fn `UpdateFootIK`
  (params (`Delta second` :type "Float (double-precision)"))
  (locals (`From Location Z` :type "Float (double-precision)") (`To Location Z` :type "Float (double-precision)") (`Left Foot Offset` :type "Float (double-precision)") (`Foot Offset Interp Speed` :type "Float (double-precision)") (`Right Foot Offset` :type "Float (double-precision)"))
  (bind (_returnvalue_x _returnvalue_y _returnvalue_z) (`KismetMathLibrary.BreakVector` (`self.K2_GetActorLocation`)))
  (bind _mesh (`self.Mesh`))
  (bind (_returnvalue_x_2 _returnvalue_y_2 _returnvalue_z_2) (`KismetMathLibrary.BreakVector` (`SceneComponent.GetSocketLocation` _mesh (`self.RightGroundSocket`))))
  (bind (_returnvalue_x_3 _returnvalue_y_3 _returnvalue_z_3) (`KismetMathLibrary.BreakVector` (`SceneComponent.GetSocketLocation` _mesh (`self.LeftGroundSocket`))))
  (set `local.From Location Z` _returnvalue_z)
  (set `local.To Location Z` (`KismetMathLibrary.FMin` _returnvalue_z_3 _returnvalue_z_2))
  (`|ExecutionSequence`
    (:`then_0`
      (bind _offset (`self.Try Get Foot Offset` _returnvalue_x_3 _returnvalue_y_3 (`local.From Location Z`) (`local.To Location Z`)))
      (set `local.Left Foot Offset` (`KismetMathLibrary.FInterpTo` (`local.Left Foot Offset`) _offset `Delta second` (`local.Foot Offset Interp Speed`))))))

(fn `UserConstructionScript`)