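; GoalObjectBP is a goal actor that signals a goal once its MBOverlappedGoal flag is true; nothing in this graph sets that flag.
; Tick polls the flag, sets GoalFlag on GameInstance_BP2, plays a sound with a five-second delayed stop, spawns Niagara at the goal mesh and calls EGoal.
; The graph never clears the flag, so this repeats every frame while true.
; Unconnected nodes for resetting the ball never run.
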(event `self.ReceiveBeginPlay`)

(event `self.ReceiveTick`
  (params (DeltaSeconds :type "Float (single-precision)"))
  (if (`self.m_bOverlappedGoal`)
    (bind _asgame_instance_bp2 (cast `/Game/Instance/GameInstance_BP2` (`GameplayStatics.GetGameInstance`)))
    (set `/Game/Instance/GameInstance_BP2.GoalFlag` true _asgame_instance_bp2)
    (`|ExecutionSequence`
      (:`then_0`
        (bind _returnvalue (`GameplayStatics.SpawnSound2D` "/Game/Sound/goallast_Cue.goallast_Cue" 1.0 1.0 0.0 null))
        (`NiagaraFunctionLibrary.SpawnSystemAtLocation` "/Game/Effect/NewNiagaraSystem.NewNiagaraSystem" (`SceneComponent.K2_GetComponentLocation` (`self.m_pGoalMesh`)) (struct) (1.0 1.0 1.0) false)
        (`KismetSystemLibrary.Delay` 5.0)
        (`AudioComponent.Stop` _returnvalue))
      (:`then_1`
        (`self.E Goal`)))))

(fn `UserConstructionScript`)