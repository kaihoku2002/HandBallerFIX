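; Player character for a team ball game with goals, handling catching, throwing, jumping and tackling.
; Tick alternates sphere-trace pickup, attaching the ball to a socket, with a downhill speed boost, and counts tackle cooldown in frames.
; Throws apply a camera-based impulse that differs in midair; goal events return the player to spawn and briefly freeze movement.
; Foot-trace IK helpers exist but are uncalled here, with right-foot offset unwired.
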(event `self.ReceiveBeginPlay`
  (`|ExecutionSequence`
    (:`then_0`
      (set `self.First Pos` (`self.K2_GetActorLocation`)))
    (:`then_1`
      ;[1 1 1] ゴール時処理　担当：坂田
      (add `/Game/BP/GoalObjectBP.E Goal` (`self.EGoal`) (delegate `EnemyGoal`)))
    (:`then_2`
      (add `/Game/BP/MyGoalObject.M Goal` (`self.MGoal`) (delegate `PlayerGoal`)))
    (:`then_3`
      ;[1 1 1] スタート時　担当：坂田
      (if (not (`/Game/Instance/GameInstance_BP2.StartFlag` (cast `/Game/Instance/GameInstance_BP2` (`GameplayStatics.GetGameInstance`) :!pure true)))
        (`CharacterMovementComponent.DisableMovement` (`self.CharacterMovement`))
        (`KismetSystemLibrary.Delay` 6.0)
        (`CharacterMovementComponent.SetMovementMode` (`self.CharacterMovement`) "MOVE_Walking" 0)))))

(event `EnemyGoal`
  ;[1 1 1] ゴール時処理　担当：坂田
  (`self.K2_SetActorLocation` (`self.First Pos`))
  (`CharacterMovementComponent.DisableMovement` (`self.CharacterMovement`))
  (`KismetSystemLibrary.Delay` 6.0)
  (`CharacterMovementComponent.SetMovementMode` (`self.CharacterMovement`) "MOVE_Walking" 0))

(event `PlayerGoal`
  ;[1 1 1] ゴール時処理　担当：坂田
  (`self.K2_SetActorLocation` (`self.First Pos`))
  (`CharacterMovementComponent.DisableMovement` (`self.CharacterMovement`))
  (`KismetSystemLibrary.Delay` 6.0)
  (`CharacterMovementComponent.SetMovementMode` (`self.CharacterMovement`) "MOVE_Walking" 0))

(event `InputAction|Throw`
  (params (Key :type "Key Structure"))
  (bind _returnvalue (`GameplayStatics.GetPlayerCameraManager` 0))
  (bind _charactermovement (`self.CharacterMovement`))
  (bind (_returnvalue_x _returnvalue_y) (`KismetMathLibrary.BreakVector` (`self.GetActorForwardVector` _returnvalue)))
  (bind (_returnvalue_roll _returnvalue_pitch _returnvalue_yaw) (`KismetMathLibrary.BreakRotator` (`SpringArmComponent.GetTargetRotation` (`self.m_pSpringArm`))))
  ;[0 1 0.1412 1 30] 投げる処理　担当：海北
  (:`Pressed`
    (if (`self.IsHolding`)
      (set `self.shooting` true)
      (set `/Game/Instance/GameInstance_BP2.Has Ball` false (cast `/Game/Instance/GameInstance_BP2` (`GameplayStatics.GetGameInstance`) :!pure true))
      (set `self.ThrowAnim` true)
      (`KismetSystemLibrary.Delay` 0.1)
      (`self.PlayAnimMontage` "/Game/Anim_Chara/throw_Montage.throw_Montage")
      (`GameplayStatics.PlaySound2D` "/Game/Sound/foley_object_throw_move_02.foley_object_throw_move_02" 1.0 1.0 0.0 null null)
      (`KismetSystemLibrary.Delay` 0.3)
      (bind _returnvalue_2 (`GameplayStatics.GetActorOfClass` "/Game/BP/Ballmain.Ballmain_C"))
      (`ActorComponent.SetActive` (`/Game/BP/Ballmain.ProjectileMovement` _returnvalue_2) false false)
      (`PrimitiveComponent.SetSimulatePhysics` (`/Game/BP/Ballmain.Sphere` _returnvalue_2) false)
      (bind _staticmesh (`/Game/BP/Ballmain.StaticMesh` _returnvalue_2))
      (`PrimitiveComponent.SetSimulatePhysics` _staticmesh true)
      (`self.SetActorEnableCollision` _returnvalue_2 true)
      (if (`NavMovementComponent.IsFalling` (`self.CharacterMovement`))
        (set `self.ThrowPower` 13000.0)
        (set `self.ThrowAngle` (`KismetMathLibrary.RotatorFromAxisAndAngle` (`KismetMathLibrary.NegateVector` (`self.GetActorRightVector` (`GameplayStatics.GetPlayerCameraManager` 0)))))
        (else
          (set `self.ThrowPower` 25000.0)
          (set `self.ThrowAngle` (`KismetMathLibrary.RotatorFromAxisAndAngle` (`KismetMathLibrary.NegateVector` (`self.GetActorRightVector` _returnvalue)) 30.0))))
      (`self.K2_SetActorRotation` (`KismetMathLibrary.MakeRotator` 0.0 0.0 _returnvalue_yaw) true)
      (`PrimitiveComponent.AddImpulse` _staticmesh (* (`KismetMathLibrary.GreaterGreater_VectorRotator` (`KismetMathLibrary.MakeVector` _returnvalue_x _returnvalue_y) (`self.ThrowAngle`)) (`self.ThrowPower`)) "None" false)
      (set `self.IsHolding` false)
      (`|ExecutionSequence`
        (:`then_0`
          (set `self.canShoot` true)
          (`KismetSystemLibrary.Delay` 1.0)
          (set `self.canShoot` false)
          (set `self.ThrowAnim` false)
          (set `self.m_bCanTackle` true)
          (set `self.CanHold` true)
          (set `self.Shooting` false))
        (:`then_1`
          (goto _label_4 :!via `Reset`))))))

(event `self.ReceiveTick`
  (params (DeltaSeconds :type "Float (single-precision)"))
  (bind _returnvalue (`self.K2_GetActorLocation`))
  (bind _charactermovement (`self.CharacterMovement`))
  (bind _charactermovement_2 (`self.CharacterMovement`))
  (bind _charactermovement_3 (`self.CharacterMovement`))
  (bind _charactermovement_4 (`self.CharacterMovement`))
  (bind (_returnvalue_x _returnvalue_y _returnvalue_z) (`KismetMathLibrary.BreakVector` (`SceneComponent.K2_GetComponentLocation` (`self.CapsuleComponent`))))
  (bind _returnvalue_2 (* (`self.GetActorUpVector`) 40.0))
  (bind _asgame_instance_bp2 (cast `/Game/Instance/GameInstance_BP2` (`GameplayStatics.GetGameInstance`) :!pure true))
  (`|ExecutionSequence`
    (:`then_0`
      (`/Engine/EditorBlueprintResources/StandardMacros.FlipFlop`
        (:`A`
          ;[0 1 0.1412 1 29] ボールを持つ処理　担当：海北
          (`|ExecutionSequence`
            (:`then_0`
              (if (`self.canShoot`)
                _
                (elif (`self.IsHolding`)
                  _
                  (elif (not (`self.m_bTackle`))
                    (bind (_outhit _returnvalue_3) (`KismetSystemLibrary.SphereTraceSingle` :`Start` (- _returnvalue _returnvalue_2) :`End` (+ _returnvalue _returnvalue_2) :`Radius` 200.0 :`TraceChannel` "TraceTypeQuery1" :`DrawTime` 0.0))
                    (if _returnvalue_3
                      (bind (_bblockinghit _binitialoverlap _time _distance _location _impactpoint _normal _impactnormal _physmat _hitactor) (`GameplayStatics.BreakHitResult` _outhit))
                      (if (`self.ActorHasTag` _hitactor "Ball")
                        (bind _output_get (set `self.Hit Actor` _hitactor))
                        (`self.K2_AttachToComponent` _output_get (`self.Mesh`) "BallCatch" "SnapToTarget" "SnapToTarget" "KeepWorld" true)
                        (bind _returnvalue_4 (`GameplayStatics.GetActorOfClass` "/Game/BP/Ballmain.Ballmain_C"))
                        (`ActorComponent.SetActive` (`/Game/BP/Ballmain.ProjectileMovement` _returnvalue_4) false false)
                        (bind _sphere (`/Game/BP/Ballmain.Sphere` _returnvalue_4))
                        (`PrimitiveComponent.SetSimulatePhysics` _sphere false)
                        (`PrimitiveComponent.SetSimulatePhysics` (`/Game/BP/Ballmain.StaticMesh` _returnvalue_4) false)
                        (`self.SetActorEnableCollision` _returnvalue_4 false)
                        (`PrimitiveComponent.SetCollisionEnabled` _sphere "PhysicsOnly")
                        (set `self.IsHolding` true)
                        (`|ExecutionSequence`
                          (:`then_0`
                            (set `self.CanHold` false)
                            (set `self.m_bCanTackle` false)
                            (set `self.canShoot` true)
                            (`GameplayStatics.PlaySound2D` "/Game/Sound/ballcatch.ballcatch" 1.0 1.0 0.0 null null)
                            (set `/Game/Instance/GameInstance_BP2.Has Ball` true _asgame_instance_bp2)
                            (set `/Game/Instance/GameInstance_BP2.Member_HasBall` true _asgame_instance_bp2))
                          (:`then_1`
                            (goto _label_4 :!via `Reset`)))))))))))
        (:`B`
          ;[0 1 0.1412] 坂を下るときに加速します　担当：海北
          (if (`NavMovementComponent.IsFalling` (`self.CharacterMovement`))
            _
            (elif (> _returnvalue_z 50.0)
              (`|ExecutionSequence`
                (:`then_0`
                  (bind _output_get_2 (set `self.Before Z` _returnvalue_z))
                  (`KismetSystemLibrary.Delay` 0.1)
                  (bind _output_get_3 (set `self.Now Z` _returnvalue_z))
                  (if (< 0.0 (- _output_get_2 _output_get_3))
                    (`|ExecutionSequence`
                      (:`then_0`
                        (`/Engine/EditorBlueprintResources/StandardMacros.DoOnce` false :!label _label
                          (:`Completed`
                            (set `CharacterMovementComponent.GravityScale` 100.0 (`self.CharacterMovement`))
                            (`/Engine/EditorBlueprintResources/StandardMacros.DoOnce` false :!label _label_2
                              (:`Completed`
                                (set `CharacterMovementComponent.MaxWalkSpeed` (* (`CharacterMovementComponent.MaxWalkSpeed` _charactermovement_3) 1.35) _charactermovement_3)
                                (set `self.Before Z` 0.0)
                                (set `self.Now Z` 0.0)
                                (`|ExecutionSequence`
                                  (:`then_0`
                                    (`KismetSystemLibrary.Delay` 1.0)
                                    (set `CharacterMovementComponent.MaxWalkSpeed` (* (`CharacterMovementComponent.MaxWalkSpeed` _charactermovement_2) 0.7408) _charactermovement_2)
                                    (set `self.NowDownAnim` false)
                                    (goto _label_2 :!via `Reset`))
                                  (:`then_1`
                                    (`KismetSystemLibrary.Delay` 0.4)
                                    (set `CharacterMovementComponent.GravityScale` 7.0 (`self.CharacterMovement`))
                                    (`KismetSystemLibrary.Delay` 1.0)
                                    (goto _label :!via `Reset`))))))))
                      (:`then_1`
                        (if (`self.NowDownAnim`)
                          _
                          (else
                            _))
                        (if (not (`self.ThrowAnim`))
                          (`self.PlayAnimMontage` "/Game/Anim_Chara/Down_Montage1.Down_Montage1")
                          (`KismetSystemLibrary.Delay` 0.5)
                          (`self.StopAnimMontage` "/Game/Anim_Chara/Down_Montage.Down_Montage")
                          (set `self.NowDownAnim` true))))))))))))
    (:`then_1`
      ;[1 1 1] タックルクールタイム　担当：坂本
      (if (`self.Cooldown_Tackle`)
        (`|ExecutionSequence`
          (:`then_0`
            (if (< (`self.Tackle_CoolTimeCnt`) (`self.Tackle Cool Time`))
              (set `self.Time_Tackle` (+ (`self.Time_Tackle`) 1))
              (if (== (mod (`self.Time_Tackle`) 60) 0)
                (set `self.Time_Tackle` 0)
                (set `self.Tackle_CoolTimeCnt` (+ (`self.Tackle_CoolTimeCnt`) 1)))
              (else
                ;;[1 1 1] 初期化
                (set `self.Tackle_CoolTimeCnt` 0)
                (set `self.Tackle_LifeFrame` 0)
                (set `self.Cooldown_Tackle` false))))
          (:`then_1`
            (if (`self.m_bTackle`)
              (if (< (`self.Tackle_LifeFrame`) 30)
                (bind _result (`/Engine/EditorBlueprintResources/StandardMacros.IncrementInt` (`self.Tackle_LifeFrame`))
                  (:`  `
                    (set `self.Tackle_LifeFrame` _result)))
                (else
                  (set `self.m_bTackle` false)
                  (set `self.Tackle_LifeFrame` 0))))))))
    (:`then_2`
      ;[0 1 0.1412] ボールを持っているかどうかで移動速度を変更　担当：海北
      (`|ExecutionSequence`
        (:`then_0`
          (if (`self.Player Recive?`)
            (`/Engine/EditorBlueprintResources/StandardMacros.DoOnce` false :!label _label_3
              (:`Completed`
                (goto _label_4 :!via `Reset`)))
            (else
              (goto _label_3 :!via `Reset`))))
        (:`then_1`
          (if (`self.Player Tackle Success?`)
            (`KismetSystemLibrary.Delay` 1.0)
            (goto _label_4 :!via `Reset`)))
        (:`then_2`
          ;[0 1 0.1412] 移動速度がおかしくなったら無理やりもどす
          (if (< (`CharacterMovementComponent.MaxWalkSpeed` _charactermovement_4) 1499.0)
            (set `CharacterMovementComponent.MaxWalkSpeed` 2000.0 _charactermovement_4)))))
    (:`then_4`
      (`/Engine/EditorBlueprintResources/StandardMacros.DoOnce` false :!label _label_4
        (:`Completed`
          (if (`self.IsHolding`)
            (set `CharacterMovementComponent.MaxWalkSpeed` 1500.0 _charactermovement)
            (else
              (set `CharacterMovementComponent.MaxWalkSpeed` 2000.0 _charactermovement)
              (if (`self.IsHolding`)
                (`KismetSystemLibrary.Delay` 1.0)
                (set `CharacterMovementComponent.MaxWalkSpeed` 1500.0 (`self.CharacterMovement`))))))))
    (:`then_5`
      ;[1 1 1] タックル関連　担当：坂本
      (if (`self.TackleStart`)
        (`|ExecutionSequence`
          (:`then_0`
            (bind _outactors (`GameplayStatics.GetAllActorsWithTag` "CPU"))
            (if (`self.OverlapedSphere`)
              (goto _label_5 :!via `Break`)
              (else
                (for _array_element _outactors :!label _label_5
                  (if (`PrimitiveComponent.IsOverlappingActor` (`self.m_pSphereComp`) _array_element)
                    (set `self.HitCPU` (cast `/Game/BP/CPUCharacterBP` _array_element :!pure true))
                    (set `self.OverlapedSphere` true)))
                ;;[1 1 1] タックル
                (set `self.OverlapedSphere` false)
                (`self.Tackle`))))
          (:`then_1`
            (`KismetSystemLibrary.Delay` 0.4)
            (set `self.TackleStart` false)))))))

(event `InputAction|Tackle`
  (params (Key :type "Key Structure"))
  ;[1 1 1] タックル関連　担当：坂本
  ;;[1 1 1] タックルインプット
  (:`Pressed`
    (set `self.TackleStart` true)))

(event `Key|Gamepad_RightShoulder`
  (params (Key :type "Key Structure"))
  ;[0 1 0.1412 1 30] ジャンプのアニメーション再生　担当：海北
  (:`Pressed`
    (if (not (`NavMovementComponent.IsFalling` (`self.CharacterMovement`)))
      (`CharacterMovementComponent.AddImpulse` (`self.CharacterMovement`) (0.0 0.0 3000.0) true)
      (`self.PlayAnimMontage` "/Game/Anim_Chara/JUMP_Montage1.JUMP_Montage1")
      (`GameplayStatics.PlaySound2D` "/Game/Sound/foley_jump_movement_throw_05.foley_jump_movement_throw_05" 1.0 1.0 0.0 null null))))

(event `Key|SpaceBar`
  (params (Key :type "Key Structure"))
  ;[0 1 0.1412 1 30] ジャンプのアニメーション再生　担当：海北
)

(fn `Tackle`
  (if (`self.Cooldown_Tackle`)
    _
    (elif (`self.m_bCanTackle`)
      (if (`self.m_bTackle`)
        _
        (elif (`self.IsHolding`)
          _
          (elif (not (`NavMovementComponent.IsFalling` (`self.CharacterMovement`)))
            (`GameplayStatics.PlaySound2D` "/Game/Sound/tacklestart.tacklestart" 1.0 1.0 0.0 null null)
            (`self.PlayAnimMontage` "/Game/Anim_Chara/takkle_Montage.takkle_Montage")
            (set `self.m_bTackle` true)
            (set `self.Cooldown_Tackle` true)))))))

(fn `TraceFromLocation`
  (params (`From Location` :type "Vector Structure") (`To Location` :type "Vector Structure"))
  (returns (Hit :type Boolean) (Location :type "Vector Structure"))
  (bind (_outhit _returnvalue) (`KismetSystemLibrary.LineTraceSingle` `From Location` `To Location` "TraceTypeQuery1"))
  (return _returnvalue (`KismetMathLibrary.SelectVector` (`.Location` (`GameplayStatics.BreakHitResult` _outhit)) (0.0 0.0 0.0) _returnvalue)))

(fn `Try Foot Trace`
  (params (`Socket Name` :type Name) (CapsuleLowerLocationZ :type "Float (double-precision)"))
  (returns (Hit :type Boolean) (`Hit Offset` :type "Float (double-precision)") (`Sinking Distance` :type "Float (double-precision)"))
  (bind _returnvalue (`SceneComponent.GetSocketLocation` (`self.Mesh`) `Socket Name`))
  (bind _z (.z _returnvalue))
  (if (> CapsuleLowerLocationZ _z)
    (bind (_hit _location) (`self.TraceFromLocation` (`KismetMathLibrary.MakeVector` (.x _returnvalue) (.y _returnvalue) CapsuleLowerLocationZ) _returnvalue))
    (return _hit (`KismetMathLibrary.SelectFloat` (- (.z _location) CapsuleLowerLocationZ) 0.0 _hit) (`KismetMathLibrary.SelectFloat` (- (.z _location) _z) 0.0 _hit))
    (else
      (return false 0.0 0.0))))

(fn `Try Get Foot Offset`
  (params (`Location X` :type "Float (double-precision)") (`Location Y` :type "Float (double-precision)") (`From Location Z` :type "Float (double-precision)") (`To Location Z` :type "Float (double-precision)"))
  (returns (Offset :type "Float (double-precision)"))
  (locals (NewLocalVar_0 :type "ARPin Object Reference"))
  (bind (_hit _location) (`self.TraceFromLocation` (`KismetMathLibrary.MakeVector` `Location X` `Location Y` `From Location Z`) (`KismetMathLibrary.MakeVector` `Location X` `Location Y` `To Location Z`)))
  (return (`KismetMathLibrary.SelectFloat` (- (.z _location) `To Location Z`) 0.0 _hit)))

(fn `UpdateActorLocationZ`
  (params (NewParam :type "Float (double-precision)"))
  (locals (DeltaSeconds_ :type "Float (double-precision)") (CapsuleLowerLocationZ :type "Float (double-precision)") (HitOffset :type "Float (double-precision)") (SinkingDistance :type "Float (double-precision)") (LocationInterpSpeed :type "Float (double-precision)" :default 50.0))
  (bind (_returnvalue_x _returnvalue_y _returnvalue_z) (`KismetMathLibrary.BreakVector` (`self.GetVelocity`)))
  (bind _capsulecomponent (`self.CapsuleComponent`))
  (bind _returnvalue (`KismetMathLibrary.FInterpTo` (`self.Interp Sinking Distance`) (`local.SinkingDistance`) 1.0 (`local.LocationInterpSpeed`)))
  (bind (_returnvalue_x_2 _returnvalue_y_2 _returnvalue_z_2) (`KismetMathLibrary.BreakVector` (`SceneComponent.K2_GetComponentLocation` _capsulecomponent)))
  (set `local.DeltaSeconds_` NewParam)
  (if (<= _returnvalue_z 0.0)
    (`|ExecutionSequence`
      (:`then_0`
        (set `local.CapsuleLowerLocationZ` (- _returnvalue_z_2 (`CapsuleComponent.CapsuleHalfHeight` _capsulecomponent))))
      (:`then_1`
        ;[1 1 1 1 37] 左あしトレース
        (bind (_hit _hit_offset _sinking_distance) (`self.Try Foot Trace` (`self.LeftGroundSocket`) (`local.CapsuleLowerLocationZ`)))
        (if (< _hit_offset (`local.HitOffset`))
          (set `local.HitOffset` _hit_offset)
          (set `local.SinkingDistance` _sinking_distance)))
      (:`then_2`
        ;[1 1 1 1 37] 右あしトレース
        (bind (_hit_2 _hit_offset_2 _sinking_distance_2) (`self.Try Foot Trace` (`self.RightGroundSocket`) (`local.CapsuleLowerLocationZ`)))
        (if (< _hit_offset_2 (`local.HitOffset`))
          (set `local.HitOffset` _hit_offset_2)
          (set `local.SinkingDistance` _sinking_distance_2)))
      (:`then_3`
        (bind _output_get (set `self.Interp Sinking Distance` _returnvalue))
        (if (> _returnvalue 0.0)
          (`self.K2_AddActorLocalOffset` (`KismetMathLibrary.MakeVector` 0.0 0.0 _output_get))
          (`CharacterMovementComponent.SetMovementMode` (`self.CharacterMovement`) "MOVE_Walking" 0))))))

(fn `UpdateFootIK`
  (params (`Delta second` :type "Float (double-precision)"))
  (locals (`From Location Z` :type "Float (double-precision)") (`To Location Z` :type "Float (double-precision)") (`Left Foot Offset` :type "Float (double-precision)") (`Foot Offset Interp Speed` :type "Float (double-precision)") (`Right Foot Offset` :type "Float (double-precision)"))
  (bind (_returnvalue_x _returnvalue_y _returnvalue_z) (`KismetMathLibrary.BreakVector` (`self.K2_GetActorLocation`)))
  (bind _mesh (`self.Mesh`))
  (bind (_returnvalue_x_2 _returnvalue_y_2 _returnvalue_z_2) (`KismetMathLibrary.BreakVector` (`SceneComponent.GetSocketLocation` _mesh (`self.RightGroundSocket`))))
  (bind (_returnvalue_x_3 _returnvalue_y_3 _returnvalue_z_3) (`KismetMathLibrary.BreakVector` (`SceneComponent.GetSocketLocation` _mesh (`self.LeftGroundSocket`))))
  (set `local.From Location Z` _returnvalue_z)
  (set `local.To Location Z` (`KismetMathLibrary.FMin` _returnvalue_z_3 _returnvalue_z_2))
  (`|ExecutionSequence`
    (:`then_0`
      (bind _offset (`self.Try Get Foot Offset` _returnvalue_x_3 _returnvalue_y_3 (`local.From Location Z`) (`local.To Location Z`)))
      (set `local.Left Foot Offset` (`KismetMathLibrary.FInterpTo` (`local.Left Foot Offset`) _offset `Delta second` (`local.Foot Offset Interp Speed`))))))

(fn `UserConstructionScript`)