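; CPU opponent character for a ball-and-goal game that chases the ball, carries it to the goal and throws it.
; Tick runs a Chase/Go/Pass state machine using AI MoveTo, sphere-trace pickup, socket attachment and impulse throws, though nothing live enters Pass.
; Capsule overlap with the player drives two-way tackles that steal the ball, with frame-counted cooldowns and GameInstance possession flags.
; Goal events return it to its start position and briefly freeze movement.
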(event `self.ReceiveTick`
  (params (DeltaSeconds :type "Float (single-precision)"))
  (bind _returnvalue (`self.K2_GetActorLocation`))
  (bind _charactermovement (`self.CharacterMovement`))
  (bind _hitplayer (`self.HitPlayer`))
  (bind _charactermovement_2 (`self.CharacterMovement`))
  (bind _hitplayer_2 (`self.HitPlayer`))
  (bind _hitplayer_3 (`self.HitPlayer`))
  (bind _returnvalue_2 (* (`self.GetActorUpVector`) 40.0))
  (bind _asgame_instance_bp2 (cast `/Game/Instance/GameInstance_BP2` (`GameplayStatics.GetGameInstance`) :!pure true))
  (bind _asgame_instance_bp2_2 (cast `/Game/Instance/GameInstance_BP2` (`GameplayStatics.GetGameInstance`) :!pure true))
  (bind _charactermovement_3 (`Character.CharacterMovement` (`self.HitPlayer`)))
  (bind _returnvalue_roll (`KismetMathLibrary.BreakRotator` (`KismetMathLibrary.FindLookAtRotation` (`self.K2_GetActorLocation` (`ActorComponent.GetOwner` (`self.Arrow1`))) (`self.K2_GetActorLocation` (`self.Goal`)))))
  (if (`self.canmove`)
    (`|ExecutionSequence`
      (:`then_0`
        (`|ExecutionSequence`
          (:`then_0`
            (switch `ECPUState` (`self.m_CPUState`)
              (:`CPUS_Chase`
                ;[0 1 0.1412] ボールを追いかける処理　担当：海北
                (bind _returnvalue_3 (`GameplayStatics.GetActorOfClass` "/Game/BP/Ballmain.Ballmain_C"))
                (bind (_returnvalue_x _returnvalue_y _returnvalue_z) (`KismetMathLibrary.BreakVector` (`SceneComponent.K2_GetComponentLocation` (`/Game/BP/Ballmain.StaticMesh` _returnvalue_3))))
                (if (> _returnvalue_z 300.0)
                  _
                  (else
                    _))
                ;;[0 1 0.1412] ボールが空中にある時の移動
                (`AIController.MoveToActor` (`AIBlueprintHelperLibrary.GetAIController` (`self.GetOwner`)) _returnvalue_3 -1.0 true false true null true)
                (`|ExecutionSequence`
                  (:`then_0`
                    ;;[0 1 0.1412] ボールを持つ処理
                    (bind (_outhits _returnvalue_4) (`KismetSystemLibrary.SphereTraceMulti` (- _returnvalue _returnvalue_2) (+ _returnvalue _returnvalue_2) 200.0 "TraceTypeQuery1" true))
                    (if _returnvalue_4
                      (for _array_element _outhits
                        (bind _asballmain (cast `/Game/BP/Ballmain` (`.HitActor` (`GameplayStatics.BreakHitResult` _array_element))))
                        (if true
                          (bind _output_get (set `self.Hit Actor` _asballmain))
                          (if (`self.Can Shoot`)
                            _
                            (elif (`self.Is holding`)
                              _
                              (elif (not (`self.Shooting`))
                                (`self.K2_AttachToComponent` _output_get (`self.Mesh`) "BallCatch" "SnapToTarget" "SnapToTarget" "KeepWorld" true)
                                (bind _returnvalue_5 (`GameplayStatics.GetActorOfClass` "/Game/BP/Ballmain.Ballmain_C"))
                                (`ActorComponent.SetActive` (`/Game/BP/Ballmain.ProjectileMovement` _returnvalue_5) false false)
                                (`PrimitiveComponent.SetSimulatePhysics` (`/Game/BP/Ballmain.Sphere` _returnvalue_5) false)
                                (`PrimitiveComponent.SetSimulatePhysics` (`/Game/BP/Ballmain.StaticMesh` _returnvalue_5) false)
                                (`self.SetActorEnableCollision` _returnvalue_5 false)
                                (`PrimitiveComponent.SetCollisionEnabled` (`/Game/BP/Ballmain.Sphere` _returnvalue_5) "PhysicsOnly")
                                (set `self.Is holding` true)
                                (`|ExecutionSequence`
                                  (:`then_0`
                                    (set `self.Can Shoot` true)
                                    (set `/Game/Instance/GameInstance_BP2.CPU_HasBall` true (cast `/Game/Instance/GameInstance_BP2` (`GameplayStatics.GetGameInstance`) :!pure true))
                                    (set `self.m_bCanTackle` false)
                                    (set `self.m_CPUState` "CPUS_Go"))
                                  (:`then_1`
                                    (goto _label_2 :!via `Reset`))))))))))))
              (:`CPUS_Go`
                ;[0 1 0.1412] ゴールに向かう処理　担当：海北
                (if (`self.PlayerCheck`)
                  (set `self.Can Shoot` true)
                  (else
                    (bind _returnvalue_6 (`GameplayStatics.GetActorOfClass` "/Game/BP/GoalJugde.GoalJugde_C"))
                    (`AIController.MoveToActor` (`AIBlueprintHelperLibrary.GetAIController` (`self.GetOwner`)) _returnvalue_6 -1.0 true false true null true)
                    (if (`/Game/BP/GoalJugde.Judge` _returnvalue_6)
                      (if (`self.Is holding`)
                        (set `self.Shooting` true)
                        (`self.K2_SetActorRotation` (`KismetMathLibrary.MakeRotator` _returnvalue_roll))
                        (`self.PlayAnimMontage` "/Game/Anim_Chara/throw_Montage.throw_Montage")
                        ;[1 1 1] ゴールに向かって投げる処理　担当：石原
                        (`KismetSystemLibrary.Delay` 0.3)
                        (bind _returnvalue_7 (`GameplayStatics.GetActorOfClass` "/Game/BP/Ballmain.Ballmain_C"))
                        (`/Engine/EditorBlueprintResources/StandardMacros.IsValid` _returnvalue_7
                          (:`Is Valid`
                            (`ActorComponent.SetActive` (`/Game/BP/Ballmain.ProjectileMovement` _returnvalue_7) false false)
                            (bind _staticmesh (`/Game/BP/Ballmain.StaticMesh` _returnvalue_7))
                            (`PrimitiveComponent.SetSimulatePhysics` _staticmesh true)
                            (`PrimitiveComponent.SetSimulatePhysics` (`/Game/BP/Ballmain.Sphere` _returnvalue_7) false)
                            (`self.SetActorEnableCollision` _returnvalue_7 true)
                            (if (not (`NavMovementComponent.IsFalling` (`self.CharacterMovement`)))
                              (`PrimitiveComponent.AddImpulse` _staticmesh (* (`KismetMathLibrary.Conv_RotatorToVector` (`SceneComponent.K2_GetComponentRotation` (`self.Arrow1`))) 20000) "None" false)
                              (set `self.Is holding` false)
                              (`|ExecutionSequence`
                                (:`then_0`
                                  (set `self.Can Shoot` false)
                                  (set `/Game/Instance/GameInstance_BP2.CPU_HasBall` false (cast `/Game/Instance/GameInstance_BP2` (`GameplayStatics.GetGameInstance`) :!pure true))
                                  (set `self.m_bCanTackle` true)
                                  (`KismetSystemLibrary.Delay` 0.2)
                                  (set `self.Shooting` false)
                                  (set `self.m_CPUState` "CPUS_Chase"))
                                (:`then_1`
                                  (goto _label_2 :!via `Reset`)))))))))))
              (:`CPUS_Pass`
                ;[1 1 1] cpuActorsの座標を取得　担当：石原
                (if (`self.Is holding`)
                  (if (`self.Can Shoot`)
                    (`self.K2_SetActorRotation` (`KismetMathLibrary.FindLookAtRotation` (`self.K2_GetActorLocation` (`ActorComponent.GetOwner` (`self.Arrow1`))) (`self.K2_GetActorLocation`)))
                    (`self.PlayAnimMontage` "/Game/Anim_Chara/throw_Montage.throw_Montage")
                    (`KismetSystemLibrary.Delay` 0.2)
                    (bind _returnvalue_8 (`GameplayStatics.GetActorOfClass` "/Game/BP/Ballmain.Ballmain_C"))
                    (`/Engine/EditorBlueprintResources/StandardMacros.IsValid` _returnvalue_8
                      (:`Is Valid`
                        (`ActorComponent.SetActive` (`/Game/BP/Ballmain.ProjectileMovement` _returnvalue_8) false false)
                        (bind _staticmesh_2 (`/Game/BP/Ballmain.StaticMesh` _returnvalue_8))
                        (`PrimitiveComponent.SetSimulatePhysics` _staticmesh_2 true)
                        (`PrimitiveComponent.SetSimulatePhysics` (`/Game/BP/Ballmain.Sphere` _returnvalue_8) false)
                        (`self.SetActorEnableCollision` _returnvalue_8 true)
                        (if (not (`NavMovementComponent.IsFalling` (`self.CharacterMovement`)))
                          (`KismetSystemLibrary.Delay` 0.2)
                          (`PrimitiveComponent.AddImpulse` _staticmesh_2 (* (`KismetMathLibrary.Conv_RotatorToVector` (`SceneComponent.K2_GetComponentRotation` (`self.Arrow1`))) (* (`self.GetDistanceTo` (`self.CPUActor`) null) 3.0)) "None" false)
                          (`KismetSystemLibrary.Delay` 0.2)
                          (set `self.Is holding` false)
                          (`|ExecutionSequence`
                            (:`then_0`
                              (set `self.Can Shoot` false)
                              (`KismetArrayLibrary.Array_Clear` (`self.CPUActors Pos`))
                              (`KismetArrayLibrary.Array_Clear` (`self.CPUTemp`))
                              (set `self.m_CPUState` "CPUS_Chase")
                              (set `/Game/Kaihoku/CPUCharacterBP.m_CPUState` "CPUS_Chase" (`self.CPUActor`)))
                            (:`then_1`
                              (goto _label_2 :!via `Reset`)))))))))))
          (:`then_1`
            ;[1 1 1] タックル関連　担当：坂田
            ;;[1 1 1] タックルクールタイム
            (if (`self.Cooldown_Tackle`)
              (`|ExecutionSequence`
                (:`then_0`
                  (if (< (`self.TackleCoolTimeCnt`) (`self.TackleCoolTime`))
                    (set `self.Time_Tackle` (+ (`self.Time_Tackle`) 1))
                    (if (== (mod (`self.Time_Tackle`) 60) 0)
                      (set `self.TackleCoolTimeCnt` (+ (`self.TackleCoolTimeCnt`) 1))
                      (set `self.Time_Tackle` 0))
                    (else
                      ;;;[1 1 1] 初期化
                      (set `self.m_iTimeCnt` 0)
                      (set `self.m_iTime` 0)
                      (set `self.Cooldown_Tackle` false))))
                (:`then_1`
                  (if (`self.m_bTackle`)
                    (if (< (`self.TackleLifeFrame`) 180)
                      (bind _result (`/Engine/EditorBlueprintResources/StandardMacros.IncrementInt` (`self.TackleLifeFrame`))
                        (:`  `
                          (set `self.TackleLifeFrame` _result)))
                      (else
                        (set `self.m_bTackle` false)
                        (set `self.TackleLifeFrame` 0))))))))
          (:`then_2`
            ;;[1 1 1] パスクールダウン
            (if (`self.Cooldown_Pass`)
              (if (< (`self.BallPassCoolTimeCnt`) (`self.BallPassCoolTime`))
                (set `self.Time_BallPass` (+ (`self.Time_BallPass`) 1))
                (if (== (mod (`self.Time_BallPass`) 60) 0)
                  (set `self.Time_BallPass` 0)
                  (set `self.BallPassCoolTimeCnt` (+ (`self.BallPassCoolTimeCnt`) 1)))
                (else
                  ;;;[1 1 1] 初期化
                  (set `self.Time_BallPass` 0)
                  (set `self.BallPassCoolTimeCnt` 0)
                  (set `self.Cooldown_Pass` false)))))
          (:`then_4`
            ;[1 1 1] タックル　担当：坂本
            (`/Engine/EditorBlueprintResources/StandardMacros.DoOnce` false :!label _label
              (:`Completed`
                (if (`self.ActorHasTag` (`self.HitPlayer`) "Player")
                  _))))
          (:`then_5`
            (if (`self.OverlapedCPUSphere`)
              (set `self.OverlapedCPUSphere` false)
              (`|ExecutionSequence`
                (:`then_0`
                  (if (`self.Cooldown_Tackle`)
                    _
                    (elif (`self.m_bCanTackle`)
                      (if (`self.Is holding`)
                        _
                        (elif (not (`NavMovementComponent.IsFalling` (`self.CharacterMovement`)))
                          (`self.PlayAnimMontage` "/Game/Anim_Chara/takkle_Montage.takkle_Montage")
                          (set `self.m_bTackle` true)
                          (set `self.Cooldown_Tackle` true)
                          (set `self.m_bCanTackle` false)
                          (if (`/Game/BP/MyCharacterBP.IsHolding` (`self.HitPlayer`))
                            (bind _returnvalue_9 (`GameplayStatics.GetActorOfClass` "/Game/BP/Ballmain.Ballmain_C"))
                            (`self.K2_DetachFromActor` _returnvalue_9 "KeepRelative" "KeepRelative" "KeepRelative")
                            (set `self.Is holding` true)
                            (`|ExecutionSequence`
                              (:`then_0`
                                (set `self.Can Shoot` true)
                                (set `self.canHaveBall` false)
                                (`self.K2_AttachToComponent` _returnvalue_9 (`self.Mesh`) "BallCatch" "SnapToTarget" "SnapToTarget" "KeepRelative" true)
                                (`self.PlayAnimMontage` _hitplayer_3 "/Game/Anim_Chara/tackle_recive_Montage.tackle_recive_Montage" 2.0 "None")
                                (bind _returnvalue_10 (`GameplayStatics.GetActorOfClass` "/Game/BP/MyCharacterBP.MyCharacterBP_C"))
                                (set `/Game/BP/MyCharacterBP.Player Recive?` true _returnvalue_10)
                                (`|ExecutionSequence`
                                  (:`then_0`
                                    (`KismetSystemLibrary.Delay` 0.2)
                                    (set `/Game/BP/MyCharacterBP.Player Recive?` false _returnvalue_10))
                                  (:`then_1`
                                    (`GameplayStatics.PlaySound2D` "/Game/Sound/tackle.tackle" 1.0 1.0 0.0 null null)
                                    (`GameplayStatics.SpawnEmitterAtLocation` "/Game/Effect/Tackle_P.Tackle_P")
                                    (`CharacterMovementComponent.AddForce` (`Character.CharacterMovement` _hitplayer_3) (* (* (`SceneComponent.GetForwardVector` (`self.Arrow2`)) 10000000.0) (`SceneComponent.GetForwardVector` (`/Game/BP/MyCharacterBP.Arrow2` (`self.HitPlayer`)))))
                                    (`|ExecutionSequence`
                                      (:`then_0`
                                        (set `/Game/BP/MyCharacterBP.IsHolding` false _hitplayer_2)
                                        (`|ExecutionSequence`
                                          (:`then_0`
                                            (set `/Game/BP/MyCharacterBP.canShoot` false _hitplayer_2)
                                            (set `Human.m_bCanTackle` true _hitplayer_2)
                                            (set `/Game/BP/MyCharacterBP.CanHold` true _hitplayer_2)
                                            (set `/Game/Instance/GameInstance_BP2.CPU_HasBall` true _asgame_instance_bp2_2)
                                            (set `/Game/Instance/GameInstance_BP2.Member_HasBall` false _asgame_instance_bp2_2)
                                            (set `/Game/Instance/GameInstance_BP2.Has Ball` false _asgame_instance_bp2_2)
                                            (if (not (`/Game/BP/MyCharacterBP.IsHolding` (`self.HitPlayer`)))
                                              (set `self.m_CPUState` "CPUS_Go")))
                                          (:`then_1`
                                            (goto _label_2 :!via `Reset`))))
                                      (:`then_1`
                                        (`KismetSystemLibrary.Delay` 0.5)
                                        (`GameplayStatics.PlaySound2D` "/Game/Sound/huttobu.huttobu" 1.0 1.0 0.0 null null)
                                        (`CharacterMovementComponent.DisableMovement` _charactermovement_3)
                                        (`KismetSystemLibrary.Delay` 1.0)
                                        (`CharacterMovementComponent.SetMovementMode` _charactermovement_3 "MOVE_Walking" 0))))))
                              (:`then_1`
                                (goto _label_2 :!via `Reset`)))))))))
                (:`then_1`
                  (if (`self.Is holding`)
                    (if (not (`self.shooting`))
                      (bind _returnvalue_11 (`GameplayStatics.GetActorOfClass` "/Game/BP/MyCharacterBP.MyCharacterBP_C"))
                      (if (`/Game/BP/MyCharacterBP.TackleStart` _returnvalue_11)
                        (if (`/Game/BP/MyCharacterBP.CanHold` _returnvalue_11)
                          (`self.PlayAnimMontage` "/Game/Anim_Chara/tackle_recive_Montage.tackle_recive_Montage")
                          (`GameplayStatics.PlaySound2D` "/Game/Sound/tackle.tackle" 1.0 1.0 0.0 null null)
                          (`GameplayStatics.SpawnEmitterAtLocation` "/Game/Effect/Tackle_P.Tackle_P" (`self.K2_GetActorLocation`))
                          (`CharacterMovementComponent.AddForce` (`self.CharacterMovement`) (* (* (`SceneComponent.GetForwardVector` (`/Game/BP/MyCharacterBP.Arrow2` (`self.HitPlayer`))) (`Human.m_TackleSpeed` (`self.HitPlayer`))) (`SceneComponent.GetForwardVector` (`self.Arrow2`))))
                          (`|ExecutionSequence`
                            (:`then_0`
                              (if (`self.Is holding`)
                                _
                                (else
                                  _))
                              (bind _returnvalue_12 (`GameplayStatics.GetActorOfClass` "/Game/BP/Ballmain.Ballmain_C"))
                              (`self.K2_DetachFromActor` _returnvalue_12 "KeepRelative" "KeepRelative" "KeepRelative")
                              (set `/Game/BP/MyCharacterBP.CanHold` false _hitplayer)
                              (set `/Game/BP/MyCharacterBP.IsHolding` true _hitplayer)
                              (`|ExecutionSequence`
                                (:`then_0`
                                  (set `/Game/BP/MyCharacterBP.canShoot` true _hitplayer)
                                  (if (not (`self.Throwed?`))
                                    (`self.K2_SetActorLocation` _returnvalue_12 (`self.K2_GetActorLocation` _returnvalue_12) false false)
                                    (`self.K2_AttachToComponent` _returnvalue_12 (`Character.Mesh` (`self.HitPlayer`)) "BallCatch" "SnapToTarget" "SnapToTarget" "KeepRelative" true)
                                    (`|ExecutionSequence`
                                      (:`then_0`
                                        (set `self.Can Shoot` false)
                                        (set `self.m_bCanTackle` true)
                                        (set `self.Is holding` false)
                                        (`|ExecutionSequence`
                                          (:`then_0`
                                            (set `self.Cooldown_Tackle` true)
                                            (set `self.m_CPUState` "CPUS_Chase")
                                            (set `/Game/Instance/GameInstance_BP2.CPU_HasBall` false _asgame_instance_bp2)
                                            (set `/Game/Instance/GameInstance_BP2.Member_HasBall` true _asgame_instance_bp2)
                                            (set `/Game/Instance/GameInstance_BP2.Has Ball` true _asgame_instance_bp2)
                                            (set `self.canmove` false)
                                            (`KismetSystemLibrary.Delay` 2.0)
                                            (set `self.canmove` true))
                                          (:`then_1`
                                            (goto _label :!via `Reset`))))
                                      (:`then_1`
                                        (bind _returnvalue_13 (`GameplayStatics.GetActorOfClass` "/Game/BP/MyCharacterBP.MyCharacterBP_C"))
                                        (set `/Game/BP/MyCharacterBP.Player Tackle Success?` true _returnvalue_13)
                                        (if (not (`/Game/BP/MyCharacterBP.IsHolding` _returnvalue_13))
                                          (set `/Game/BP/MyCharacterBP.Player Tackle Success?` true _returnvalue_13)
                                          (set `CharacterMovementComponent.MaxWalkSpeed` 1500.0 (`Character.CharacterMovement` _returnvalue_13)))))))
                                (:`then_1`
                                  (goto _label :!via `Reset`))))
                            (:`then_1`
                              (`KismetSystemLibrary.Delay` 0.5)
                              (`GameplayStatics.PlaySound2D` "/Game/Sound/huttobu.huttobu" 1.0 1.0 0.0 null null)
                              (`CharacterMovementComponent.DisableMovement` _charactermovement)
                              (set `self.OverlapedCPUSphere` false)
                              (`KismetSystemLibrary.Delay` 1.5)
                              (`CharacterMovementComponent.SetMovementMode` _charactermovement "MOVE_Walking" 0)
                              (goto _label_2 :!via `Reset`)))))))))))))
      (:`then_1`
        ;[1 1 1] スタート時
        (if (not (`/Game/Instance/GameInstance_BP2.StartFlag` (cast `/Game/Instance/GameInstance_BP2` (`GameplayStatics.GetGameInstance`) :!pure true)))
          (`CharacterMovementComponent.DisableMovement` (`self.CharacterMovement`))
          (`KismetSystemLibrary.Delay` 6.0)
          (`CharacterMovementComponent.SetMovementMode` (`self.CharacterMovement`) "MOVE_Walking" 0)))
      (:`then_2`
        (bind _returnvalue_14 (`GameplayStatics.GetActorOfClass` "/Game/BP/MyCharacterBP.MyCharacterBP_C"))
        (if (`PrimitiveComponent.IsOverlappingActor` (`self.CapsuleComponent`) _returnvalue_14)
          (set `self.OverlapedCPUSphere` true)
          (else
            (set `self.OverlapedCPUSphere` false))))
      (:`then_4`
        ;[0 1 0.1412] 移動スピードを変更　担当：海北
        (`/Engine/EditorBlueprintResources/StandardMacros.DoOnce` false :!label _label_2
          (:`Completed`
            (if (`self.Is holding`)
              (set `CharacterMovementComponent.MaxWalkSpeed` 1500.0 _charactermovement_2)
              (else
                (set `CharacterMovementComponent.MaxWalkSpeed` 2000.0 _charactermovement_2)))))))))

(event `self.ReceiveBeginPlay`
  (bind _asgame_instance_bp2 (cast `/Game/Instance/GameInstance_BP2` (`GameplayStatics.GetGameInstance`) :!pure true))
  (`|ExecutionSequence`
    (:`then_0`
      ;[1 1 1] ゴールオブジェクトゲッチュー　担当：坂田
      (bind _returnvalue (`GameplayStatics.GetActorOfClass` "/Game/BP/GoalObjectBP.GoalObjectBP_C"))
      (set `self.goal` _returnvalue)
      (set `/Game/Instance/GameInstance_BP2.CPU_HasBall` false _asgame_instance_bp2)
      (set `/Game/Instance/GameInstance_BP2.Member_HasBall` false _asgame_instance_bp2)
      (set `/Game/Instance/GameInstance_BP2.Has Ball` false _asgame_instance_bp2))
    (:`then_1`
      ;[1 1 1] ゴール時処理　担当：坂田
      (set `self.First Pos` (`self.K2_GetActorLocation`)))
    (:`then_2`
      (add `/Game/BP/MyGoalObject.M Goal` (`self.MGoal`) (delegate `Player Goal`)))
    (:`then_3`
      (add `/Game/BP/GoalObjectBP.E Goal` (`self.EGoal`) (delegate `Enemy Goal`)))
    (:`then_4`
      (bind _outactors (`GameplayStatics.GetAllActorsOfClass` "/Game/BP/MyCharacterBP.MyCharacterBP_C"))
      (for (_array_element _array_index) _outactors
        (if (== _array_index 0)
          (set `self.HitPlayer` _array_element))))))

(event `Player Goal`
  ;[1 1 1] ゴール時処理　担当：坂田
  (`self.K2_SetActorLocation` (`self.First Pos`))
  (`CharacterMovementComponent.DisableMovement` (`self.CharacterMovement`))
  (`KismetSystemLibrary.Delay` 6.0)
  (`CharacterMovementComponent.SetMovementMode` (`self.CharacterMovement`) "MOVE_Walking" 0)
  (set `self.m_CPUState` "CPUS_Chase"))

(event `Enemy Goal`
  ;[1 1 1] ゴール時処理　担当：坂田
  (`self.K2_SetActorLocation` (`self.First Pos`))
  (`CharacterMovementComponent.DisableMovement` (`self.CharacterMovement`))
  (`KismetSystemLibrary.Delay` 6.0)
  (`CharacterMovementComponent.SetMovementMode` (`self.CharacterMovement`) "MOVE_Walking" 0)
  (set `self.m_CPUState` "CPUS_Chase"))

(fn `Overlap Member`
  (bind _returnvalue (`GameplayStatics.GetActorOfClass` null))
  (if (< (`self.GetDistanceTo` _returnvalue) 300.0)
    (set `self.Member Check` true)))

(fn `Overlap Player`
  (locals (NewLocalVar_0 :type Boolean))
  (bind _returnvalue (`GameplayStatics.GetActorOfClass` "/Game/BP/MyCharacterBP.MyCharacterBP_C"))
  (if (< (`self.GetDistanceTo` _returnvalue) 300.0)
    (set `self.PlayerCheck` true)))

(fn `UserConstructionScript`)